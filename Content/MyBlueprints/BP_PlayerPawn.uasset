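; BP_PlayerPawn is a player pawn with basic planar movement and yaw rotation driven by project input axes.
; Each Tick, it scales the MoveForward, MoveRight and SpinYaw axis values by linear or angular velocity and delta time for frame-rate-independent motion.
; The result feeds a single swept AddActorLocalTransform, so movement follows the pawn's own orientation and respects collision.
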(event EventTick
  (params (DeltaSeconds :type Float%20%28single-precision%29))
  (bind _linvel (Variables|Default|GetlinVel))
  (bind _returnvalue (* _linvel DeltaSeconds))
  ;[1 1 1] Basic movement using axis inputs set in project settings
  (Class|Actor|AddActorLocalTransform (Math|Transform|MakeTransform (Math|Vector|MakeVector (* _returnvalue (Input|AxisValues|GetMoveForward)) (* _returnvalue (Input|AxisValues|GetMoveRight)) 0.0) (Math|Rotator|MakeRotator 0.0 0.0 (* (* (Variables|Default|GetangVel) DeltaSeconds) (Input|AxisValues|GetSpinYaw))) (Transformation|GetActorScale3D)) true false))

(fn ConstructionScript)