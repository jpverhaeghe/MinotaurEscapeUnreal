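; BP_PlayerAsCamera is a player Blueprint, named as a camera stand-in, with basic movement and a jump.
; Each Tick applies a swept local transform from forward, right and yaw axis inputs, scaled by linear or angular speed and delta time.
; Jump is a direct, unswept local Z offset by JumpForce on press, with another offset derived from JumpForce on release, without physics.
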(event EventTick
  (params (DeltaSeconds :type Float%20%28single-precision%29))
  (bind _linvel (Variables|Default|GetlinVel))
  (bind _returnvalue (* _linvel DeltaSeconds))
  ;[1 1 1] Basic movement using axis inputs set in project settings
  (Class|Actor|AddActorLocalTransform (Math|Transform|MakeTransform (Math|Vector|MakeVector (* _returnvalue (Input|AxisValues|GetMoveForward)) (* _returnvalue (Input|AxisValues|GetMoveRight)) 0.0) (Math|Rotator|MakeRotator 0.0 0.0 (* (* (Variables|Default|GetangVel) DeltaSeconds) (Input|AxisValues|GetSpinYaw))) "1.000000,1.000000,1.000000") true false))

(event Input|ActionEvents|InputActionInputAction_Jump
  (params (Key :type Key%20Structure))
  (bind _jumpforce (Variables|Default|GetjumpForce))
  ;[1 1 1] Press space to Jump using force
  (:Pressed
    (Class|Actor|AddActorLocalTransform (Math|Transform|MakeTransform (Math|Vector|MakeVector 0.0 0.0 _jumpforce) "0, 0, 0" "1.000000,1.000000,1.000000") false false))
  (:Released
    (bind _result (Math|Float|NegateFloat _jumpforce)
      (:%20%20
        (Class|Actor|AddActorLocalTransform (Math|Transform|MakeTransform (Math|Vector|MakeVector 0.0 0.0 _result) "0, 0, 0" "1.000000,1.000000,1.000000") false false)))))

(fn ConstructionScript)