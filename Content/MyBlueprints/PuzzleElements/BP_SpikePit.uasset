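; BP_SpikePit is a puzzle hazard that kills the Hero on overlap or gets filled by a moveable box.
; A Hero overlap starts a short timer to KillHero, which plays a Wilhelm scream, zeroes the Hero's speed and destroys it.
; A box overlap hides the box, swaps the pit's material to a filled look and disables collision on both, neutralizing the hazard.
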(event Collision|EventActorBeginOverlap
  (params (OtherActor :type Actor%20Object%20Reference))
  ;[1 1 1] If it is the Hero, kill it
  (bind _asbp_hero (Utilities|Casting|CastToBP_Hero OtherActor)
    (:then
      (Variables|Default|SetCollidedHero _asbp_hero)
      (Utilities|Time|SetTimerbyFunctionName 0 "KillHero" 0.75))
    (:CastFailed
      ;[1 1 1] If it is a box, hide it, change the material to look like it is in the hole and disable both objects
      (bind _asbp_moveable_box (Utilities|Casting|CastToBP_MoveableBox OtherActor))
      (bind _output_get (Variables|Default|SetMoveableBox _asbp_moveable_box))
      (Rendering|SetActorHiddenInGame _output_get true)
      (Collision|SetActorEnableCollision _output_get false)
      (Rendering|Material|SetMaterial (Variables|Default|GetPitArea) 0 (Variables|Default|GetFillMaterial))
      (Collision|SetActorEnableCollision false))))

(fn ConstructionScript)

(fn KillHero
  (Audio|Components|Audio|Play (Variables|Default|GetVOXScrm_Wilhelm_scream__ID_0477__BSB) 0.0)
  (Variables|/Game/MyBlueprints/PuzzleElements/BP_Hero.BP_Hero_C|SetSpeed (Variables|Default|GetCollidedHero) 0.0)
  (Actor|DestroyActor (Variables|Default|GetCollidedHero))
  (Variables|Default|SetCollidedHero 0))