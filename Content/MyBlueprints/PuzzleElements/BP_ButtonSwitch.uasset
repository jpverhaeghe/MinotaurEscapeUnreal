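; BP_ButtonSwitch is a puzzle button that spawns a BP_Hero at the level's BP_HeroStartPoint.
; A box overlap enables input when a BP_PlayerPawn enters; any actor leaving disables it.
; Pressing F lowers the button, plays a click sound and spawns the hero, unless one exists or the button is down.
; A one-second timer calls WaitRelease to raise the button and clear the pressed state.
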(event OnComponentBeginOverlap(Box)
  (params (OverlappedComponent :type Primitive%20Component%20Object%20Reference) (OtherActor :type Actor%20Object%20Reference) (OtherComp :type Primitive%20Component%20Object%20Reference) (OtherBodyIndex :type Integer) (bFromSweep :type Boolean) (SweepResult :type Hit%20Result%20Structure%20%28by%20ref%29))
  ;[1 1 1] Set up input if the player is nearby, disable if they leave the button area
  (if (Utilities|ClassIsChildOf (Utilities|GetClass OtherActor) "/Game/MyBlueprints/BP_PlayerPawn.BP_PlayerPawn_C")
    (Input|EnableInput (Game|GetPlayerController 0))))

(event OnComponentEndOverlap(Box)
  (params (OverlappedComponent :type Primitive%20Component%20Object%20Reference) (OtherActor :type Actor%20Object%20Reference) (OtherComp :type Primitive%20Component%20Object%20Reference) (OtherBodyIndex :type Integer))
  ;[1 1 1] Set up input if the player is nearby, disable if they leave the button area
  (if true
    (Input|DisableInput (Game|GetPlayerController 0))))

(event EventBeginPlay
  ;[1 1 1] Grab the hero start point, there should only be one
  (bind _returnvalue (Actor|GetActorOfClass "/Game/MyBlueprints/PuzzleElements/BP_HeroStartPoint.BP_HeroStartPoint_C"))
  (Variables|Default|SetHeroStartPoint _returnvalue))

(event Input|KeyboardEvents|F
  (params (Key :type Key%20Structure :default "None"))
  ;[1 1 1] When the button is pressed, spawn the hero (can we make this generic so we can re-use it?)
  (:Pressed
    (if (not (or (Utilities|IsValid (Variables|Default|GetSpawnedHero)) (Variables|Default|GetPressed)))
      (Transformation|AddLocalOffset (Variables|Default|GetButton) "0.000000,0.000000,-15.000000" false false)
      (Variables|Default|SetPressed true)
      (Audio|Components|Audio|Play (Variables|Default|Get414438__inspectorj__light-pulley-switch-on-c) 0.0)
      (bind _returnvalue (Game|SpawnActorfromClass "/Game/MyBlueprints/PuzzleElements/BP_Hero.BP_Hero_C" (Transformation|GetActorTransform (Variables|Default|GetHeroStartPoint)) "Undefined" 0 0))
      (Variables|Default|SetSpawnedHero _returnvalue)
      (Utilities|Time|SetTimerbyFunctionName 0 "WaitRelease" 1.0))))

(fn ConstructionScript)

(fn WaitRelease
  (Transformation|AddLocalOffset (Variables|Default|GetButton) "0.000000,0.000000,15.000000" false false)
  (Variables|Default|SetPressed false))