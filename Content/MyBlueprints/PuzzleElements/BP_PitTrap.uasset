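; BP_PitTrap is a puzzle pit that kills the Hero or gets filled by a pushed box.
; On overlap, the Hero screams and a short timer calls its KillHero function.
; A BP_BoxMoveable is hidden, the pit swaps to a fill material, both lose collision, and the box stores a reference to the pit.
; RemoveBox restores the pit's material and collision, then destroys the stored box.
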(event Collision|EventActorBeginOverlap
  (params (OtherActor :type Actor%20Object%20Reference))
  ;[1 1 1] If it is the Hero, kill it
  (bind _asbp_hero (Utilities|Casting|CastToBP_Hero OtherActor)
    (:then
      (Default|PlayScream _asbp_hero)
      (Utilities|Time|SetTimerbyFunctionName _asbp_hero "KillHero" 0.75))
    (:CastFailed
      ;[1 1 1] If it is a box, hide it, change the material to look like it is in the hole and disable both objects
      (bind _asbp_box_moveable (Utilities|Casting|CastToBP_BoxMoveable OtherActor))
      (bind _output_get (Variables|Default|SetBoxInPit _asbp_box_moveable))
      (Rendering|SetActorHiddenInGame _output_get true)
      (Collision|SetActorEnableCollision _output_get false)
      (Rendering|Material|SetMaterial (Variables|Default|GetPitArea) 0 (Variables|Default|GetFillMaterial))
      (Collision|SetActorEnableCollision false)
      (Variables|/Game/MyBlueprints/PuzzleElements/BP_BoxMoveable.BP_BoxMoveable_C|SetPitTrap _output_get self))))

(fn ConstructionScript)

(fn RemoveBox
  (Rendering|Material|SetMaterial (Variables|Default|GetPitArea) 0 (Variables|Default|GetPitMaterial))
  (Collision|SetActorEnableCollision true)
  (Actor|DestroyActor (Variables|Default|GetBoxInPit))
  (Variables|Default|SetBoxInPit 0))