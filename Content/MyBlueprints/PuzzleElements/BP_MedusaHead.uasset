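; Medusa head puzzle statue whose sight beam turns the player pawn or hero to stone.
; While sight is enabled and not rotating, Tick box-traces forward, petrifies valid hits and shortens the Niagara beam to the hit actor.
; An optional timer interpolates the statue base through yaw steps, respawning the beam after each turn; otherwise the beam respawns on a loop.
; A pressure plate flag blocks beam spawning, while a separate flag gates sight and rotation.
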(event EventTick
  (params (DeltaSeconds :type Float%20%28single-precision%29))
  (bind _statuebase (Variables|Default|GetStatueBase))
  (bind _medusahead (Variables|Default|GetMedusaHead))
  (bind _rotateto (Variables|Default|GetRotateTo))
  (bind _returnvalue (Transformation|GetWorldLocation _medusahead))
  (bind _returnvalue_2 (Transformation|GetWorldRotation _medusahead))
  (bind _returnvalue_3 (Transformation|GetWorldRotation _statuebase))
  (bind _returnvalue_4 (Math|Interpolation|RInterpTo _returnvalue_3 _rotateto DeltaSeconds 2e+01))
  ;[1 1 1] Only cast if we are turned on and not rotating
  (if (Variables|Default|GetStoneSightEnabled)
    (if (Variables|Default|GetRotating)
      ;[1 1 1] Rotate using interpolation to the new rotation angle and spawn the next beam
      (Transformation|SetWorldRotation _statuebase _returnvalue_4 false false)
      (if (Utilities|Operators|EqualEqual _rotateto _returnvalue_4 0.0005)
        (Variables|Default|SetRotating false)
        (CallFunction|SpawnBeam)
        (CallFunction|UpdateBeam :!label _label))
      (else
        ;[1 1 1] Cast out to see if this can turn something to stone
        (bind _output_get (Variables|Default|SetEndBeam (+ _returnvalue (* (Math|Vector|GetForwardVector _returnvalue_2) (Variables|Default|GetSightDistance)))))
        (bind (_outhit _returnvalue_5) (Class|KismetSystemLibrary|BoxTraceSingleforObjects _returnvalue _output_get "10.000000,10.000000,10.000000" _returnvalue_2 (Variables|Default|GetObjectsToFreeze) false 0 "None" true))
        (if _returnvalue_5
          (CallFunction|TurntoStone _outhit)
          (goto _label)
          (else
            (goto _label)))))))

(event EventBeginPlay
  ;[1 1 1] Set up timer rotation if it is turned on, and if not, set up beam to loop
  (if (Variables|Default|GetRotateOnTimer)
    (Utilities|Time|SetTimerbyFunctionName 0 "RotateMedusa" (Variables|Default|GetTimeBetweenRotations) true)
    (CallFunction|SpawnBeam)
    (else
      (Utilities|Time|SetTimerbyFunctionName 0 "SpawnBeam" 2.0 true))))

(fn ConstructionScript
  ;[1 1 1] Set up the initial rotation
  (Transformation|SetActorRotation (Variables|Default|GetInitialRotation)))

(fn RotateMedusa
  (bind _statuebase (Variables|Default|GetStatueBase))
  (bind _returnvalue (Transformation|GetWorldRotation _statuebase))
  ;[1 1 1] Set the up the rotation which is performed in the main tick
  (Variables|Default|SetRotateTo (Math|Rotator|MakeRotator (.roll _returnvalue) (.pitch _returnvalue) (+ (.yaw _returnvalue) (Variables|Default|GetRotationAngle))))
  (Variables|Default|SetRotating true))

(fn TurntoStone
  (params (HitTarget :type Hit%20Result%20Structure))
  (bind _hitactor (Collision|BreakHitResult HitTarget))
  ;[1 1 1] If it is the player, turn them to stone for a bit
  (bind _asbp_player_pawn (Utilities|Casting|CastToBP_PlayerPawn _hitactor)
    (:then
      (Default|TurntoStone _asbp_player_pawn))
    (:CastFailed
      ;[1 1 1] If it is the hero, turn it to stone then it dies
      (bind _asbp_hero (Utilities|Casting|CastToBP_Hero _hitactor)
        (:then
          (Default|TurntoStone _asbp_hero))
        (:CastFailed
          _))))
  ;[1 1 1] In any case, stop the beam from going past the actor it hit
  (Variables|Default|SetEndBeam (Transformation|GetWorldLocation (Variables|/Script/Engine.Actor|GetRootComponent _hitactor))))

(fn SpawnBeam
  (bind _medusahead (Variables|Default|GetMedusaHead))
  ;[1 1 1] Create a beam showing where this medusa is dangerous - if not stopped by a pressure plate
  (if (not (Variables|Default|GetStoppedByPlate))
    (bind _returnvalue (Niagara|SpawnSystematLocation "/Game/MyParticleSystems/P_MedusaBeam.P_MedusaBeam" (Transformation|GetWorldLocation _medusahead) (Transformation|GetWorldRotation _medusahead)))
    (Variables|Default|SetCurrentBeam _returnvalue)))

(fn UpdateBeam
  (Niagara|SetNiagaraVariable(Vector3) (Variables|Default|GetCurrentBeam) "BeamEnd" (Variables|Default|GetEndBeam)))