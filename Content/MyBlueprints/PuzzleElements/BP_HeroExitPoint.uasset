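; BP_HeroExitPoint is the puzzle's goal actor, which marks a hero as escaped when it overlaps.
; The overlap casts to BP_Hero, prints a debug message for other actors, and stores the hero before starting a one-second timer.
; EndMovement then adjusts the hero's pitch, zeroes its speed and sets Escaped.
; A second timer calls RemoveHero a second later to destroy the hero.
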(event Collision|EventActorBeginOverlap
  (params (OtherActor :type Actor%20Object%20Reference))
  ;[1 1 1] When the hero gets here, the puzzle is solved! Stop the hero and mark it as escaped
  (bind _asbp_hero (Utilities|Casting|CastToBP_Hero OtherActor)
    (:then
      (Variables|Default|SetCollidedHero _asbp_hero)
      (Utilities|Time|SetTimerbyFunctionName 0 "EndMovement" 1.0))
    (:CastFailed
      (Development|PrintString "Not a hero BP" true false "(R=0.588542,G=0.000000,B=0.032264,A=1.000000)" 1e+01))))

(fn ConstructionScript)

(fn EndMovement
  (bind _collidedhero (Variables|Default|GetCollidedHero))
  (Transformation|AddActorLocalRotation _collidedhero (Math|Rotator|MakeRotator 0.0 (- 1.0 (.pitch (Transformation|GetActorRotation _collidedhero))) 0.0) false false)
  (Variables|/Game/MyBlueprints/PuzzleElements/BP_Hero.BP_Hero_C|SetSpeed _collidedhero 0.0)
  (Variables|/Game/MyBlueprints/PuzzleElements/BP_Hero.BP_Hero_C|Setescaped _collidedhero true)
  (Utilities|Time|SetTimerbyFunctionName 0 "RemoveHero" 1.0))

(fn RemoveHero
  (Actor|DestroyActor (Variables|Default|GetCollidedHero)))