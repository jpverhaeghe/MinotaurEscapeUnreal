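; Puzzle switch that spawns a moveable box at the level's BP_BoxSpawnPoint when the player presses F nearby.
; A box trigger enables input when the player pawn enters and disables it when any actor leaves.
; Each press lowers the button, plays a sound and locks it until a timer calls WaitRelease.
; Spawned boxes are capped at NumBoxes, with the oldest removed through its PitTrap if set, otherwise destroyed.
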(event OnComponentBeginOverlap(Box)
  (params (OverlappedComponent :type Primitive%20Component%20Object%20Reference) (OtherActor :type Actor%20Object%20Reference) (OtherComp :type Primitive%20Component%20Object%20Reference) (OtherBodyIndex :type Integer) (bFromSweep :type Boolean) (SweepResult :type Hit%20Result%20Structure%20%28by%20ref%29))
  ;[1 1 1] Set up input if the player is nearby, disable if they leave the button area
  (if (Utilities|ClassIsChildOf (Utilities|GetClass OtherActor) "/Game/MyBlueprints/BP_PlayerPawn.BP_PlayerPawn_C")
    (Input|EnableInput (Game|GetPlayerController 0))))

(event OnComponentEndOverlap(Box)
  (params (OverlappedComponent :type Primitive%20Component%20Object%20Reference) (OtherActor :type Actor%20Object%20Reference) (OtherComp :type Primitive%20Component%20Object%20Reference) (OtherBodyIndex :type Integer))
  ;[1 1 1] Set up input if the player is nearby, disable if they leave the button area
  (if true
    (Input|DisableInput (Game|GetPlayerController 0))))

(event EventBeginPlay
  ;[1 1 1] Grab the hero start point, there should only be one
  (bind _returnvalue (Actor|GetActorOfClass "/Game/MyBlueprints/PuzzleElements/BP_BoxSpawnPoint.BP_BoxSpawnPoint_C"))
  (Variables|Default|SetBoxSpawnPoint _returnvalue))

(event Input|KeyboardEvents|F
  (params (Key :type Key%20Structure :default "None"))
  (bind _boxspawnpoint (Variables|Default|GetBoxSpawnPoint))
  (bind _boxesspawned (Variables|Default|GetBoxesSpawned))
  (bind _returnvalue (Transformation|GetActorTransform _boxspawnpoint))
  (bind _output (Utilities|Array|Get(acopy) _boxesspawned))
  (bind (_location _rotation) (Math|Transform|BreakTransform _returnvalue))
  (bind _pittrap (Variables|/Game/MyBlueprints/PuzzleElements/BP_BoxMoveable.BP_BoxMoveable_C|GetPitTrap _output))
  ;[1 1 1] Only spawn if not already pressed
  (:Pressed
    (if (not (Variables|Default|GetPressed))
      ;[1 1 1] If there aren't enough boxes, remove the first one
      (if (< (Utilities|Array|Length _boxesspawned) (Variables|Default|GetNumBoxes))
        _
        (else
          (if (Utilities|IsValid _pittrap)
            (Default|RemoveBox _pittrap)
            (else
              (Actor|DestroyActor _output)))
          (Utilities|Array|RemoveIndex _boxesspawned)))
      ;[1 1 1] Create a new box now that we can (if one was removed and the button is not in pressed mode)
      (Transformation|AddLocalOffset (Variables|Default|GetButton) "0.000000,0.000000,-15.000000" false false)
      (Variables|Default|SetPressed true)
      (Audio|Components|Audio|Play (Variables|Default|Get414438__inspectorj__light-pulley-switch-on-c) 0.0)
      (bind _returnvalue_2 (Game|SpawnActorfromClass "/Game/MyBlueprints/PuzzleElements/BP_BoxMoveable.BP_BoxMoveable_C" (Math|Transform|MakeTransform _location _rotation "0.800000,0.800000,0.800000") "AdjustIfPossibleButAlwaysSpawn" 0 0))
      (Utilities|Array|Add (Variables|Default|GetBoxesSpawned) _returnvalue_2)
      (Utilities|Time|SetTimerbyFunctionName 0 "WaitRelease" 1.0))))

(fn ConstructionScript)

(fn WaitRelease
  (Transformation|AddLocalOffset (Variables|Default|GetButton) "0.000000,0.000000,15.000000" false false)
  (Variables|Default|SetPressed false))