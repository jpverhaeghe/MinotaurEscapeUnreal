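; BP_Hero is a puzzle-element character that walks toward an exit and can be turned to stone.
; SetHeroExitPoint stores the exit and faces the hero at it once; Tick then pushes it along local X by Speed.
; TurnToStone runs once, zeroing Speed, swapping to a stone material, playing a Wilhelm scream and starting a named timer that calls KillHero to destroy the actor.
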(event EventTick
  (params (DeltaSeconds :type Float%20%28single-precision%29))
  ;[1 1 1] Move towards the exit if we are not stone
  (if (not (and (AI|Components|NavMovement|IsFalling (Variables|Character|GetCharacterMovement)) (Variables|Default|GetisStone)))
    (Class|Actor|AddActorLocalTransform (Math|Transform|MakeTransform (Math|Vector|MakeVector (* DeltaSeconds (Variables|Default|GetSpeed)) 0.0 0.0) "0, 0, 0" "0.500000,0.500000,0.500000") false false)))

(fn ConstructionScript)

(fn RotateTowardsExit
  (Transformation|SetActorRotation (Math|Rotator|FindLookatRotation (Transformation|GetActorLocation) (Transformation|GetActorLocation (Variables|Default|GetHeroExit)))))

(fn TurntoStone
  ;[1 1 1] Only turn to stone if not already stone
  (if (not (Variables|Default|GetIsStone))
    ;[1 1 1] Turn the hero to stoneby setting the material, playing the death scream and set kill function with timer
    (Variables|Default|SetIsStone true)
    (Variables|Default|SetSpeed 0.0)
    (Rendering|Material|SetMaterial (Variables|Character|GetMesh) 0 (Variables|Default|GetStoneMaterial))
    (CallFunction|PlayScream)
    (Utilities|Time|SetTimerbyFunctionName 0 "KillHero" (Variables|Default|GetTime%20as%20Stone))))

(fn KillHero
  (Variables|Default|SetSpeed 0.0)
  (Actor|DestroyActor))

(fn PlayScream
  (Audio|Components|Audio|Play (Variables|Default|GetVOXScrm_Wilhelm_scream__ID_0477__BSB) 0.0))

(fn SetHeroExitPoint
  (params (HeroExit :type BP%20Hero%20Exit%20Point%20Object%20Reference))
  ;[1 1 1] Set up access to the exit point and rotate towards it
  (Variables|Default|SetHeroExit HeroExit)
  (CallFunction|RotateTowardsExit))