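; BP_Room is a level-generation room tile that builds its own walls and can turn its floor to lava.
; DrawWalls switches on RoomType, whose compass letters mark open sides, spawning scaled cube StaticMeshActors on closed sides, sized and placed from the Floor's scale.
; Spawned walls take the given material, attach to the room and are stored in Walls for DestryoWalls to remove.
; SetLava swaps the floor material by percentage chance when allowed.
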(fn ConstructionScript)

(fn DrawWalls
  (params (WallMaterial :type Material%20Instance%20Object%20Reference))
  (bind _floor (Variables|Default|GetFloor))
  (bind _roomtype (Variables|Default|GetRoomType))
  (bind _relativescale3d (Variables|/Script/Engine.SceneComponent|GetRelativeScale3D _floor))
  ;[1 1 1] Set up width and height value and begin wall creation
  (Variables|Default|SetWallMaterial WallMaterial)
  (bind _output_get (Variables|Default|SetRoomWidth (* (.x _relativescale3d) 1e+02)))
  (bind _output_get_2 (Variables|Default|SetRoomHeight (* (.y _relativescale3d) 1e+02)))
  ;[1 1 1] Make North wall
  (switch Utilities|FlowControl|Switch|SwitchonRoomType _roomtype
    (:NewEnumerator0
      (bind _returnvalue (Game|SpawnActorfromClass "/Script/Engine.StaticMeshActor" (Math|Transform|MakeTransform (Math|Vector|MakeVector 0.0 (|(5-(dim/2)) _output_get_2) 0.0) "0, 0, 0" (Math|Vector|MakeVector (.x _relativescale3d) 0.1 4.0)) "Undefined" 0 0 :!label _label))
      (Transformation|SetMobility _returnvalue "Stationary")
      (Components|StaticMesh|SetStaticMesh (Variables|/Script/Engine.StaticMeshActor|GetStaticMeshComponent _returnvalue) "/Game/Shapes/Shape_Cube.Shape_Cube")
      (Rendering|Material|SetMaterial (Variables|/Script/Engine.StaticMeshActor|GetStaticMeshComponent _returnvalue) 0 (Variables|Default|GetWallMaterial))
      (Transformation|AttachActorToActor _returnvalue self "None" "KeepRelative" "KeepRelative" "KeepRelative" true)
      (Utilities|Array|Add (Variables|Default|GetWalls) _returnvalue))
    (:NewEnumerator1
      _)
    (:NewEnumerator2
      _)
    (:NewEnumerator3
      _)
    (:NewEnumerator4
      _)
    (:NewEnumerator5
      (goto _label))
    (:NewEnumerator6
      _)
    (:NewEnumerator7
      _)
    (:NewEnumerator8
      _)
    (:NewEnumerator9
      (goto _label))
    (:NewEnumerator10
      (goto _label))
    (:NewEnumerator11
      (goto _label))
    (:NewEnumerator12
      _)
    (:NewEnumerator13
      (goto _label))
    (:NewEnumerator14
      (goto _label))
    (:NewEnumerator15
      (goto _label)))
  ;[1 1 1] Make East wall
  (switch Utilities|FlowControl|Switch|SwitchonRoomType _roomtype
    (:NewEnumerator0
      _)
    (:NewEnumerator1
      _)
    (:NewEnumerator2
      _)
    (:NewEnumerator3
      _)
    (:NewEnumerator4
      (bind _returnvalue_2 (Game|SpawnActorfromClass "/Script/Engine.StaticMeshActor" (Math|Transform|MakeTransform (Math|Vector|MakeVector (|((dim/2)-5) _output_get) 0.0 0.0) "0, 0, 0" (Math|Vector|MakeVector 0.1 (.y _relativescale3d) 4.0)) "Undefined" 0 0 :!label _label_2))
      (Transformation|SetMobility _returnvalue_2 "Stationary")
      (Components|StaticMesh|SetStaticMesh (Variables|/Script/Engine.StaticMeshActor|GetStaticMeshComponent _returnvalue_2) "/Game/Shapes/Shape_Cube.Shape_Cube")
      (Rendering|Material|SetMaterial (Variables|/Script/Engine.StaticMeshActor|GetStaticMeshComponent _returnvalue_2) 0 (Variables|Default|GetWallMaterial))
      (Transformation|AttachActorToActor _returnvalue_2 self "None" "KeepRelative" "KeepRelative" "KeepRelative" true)
      (Utilities|Array|Add (Variables|Default|GetWalls) _returnvalue_2))
    (:NewEnumerator5
      _)
    (:NewEnumerator6
      _)
    (:NewEnumerator7
      (goto _label_2))
    (:NewEnumerator8
      (goto _label_2))
    (:NewEnumerator9
      _)
    (:NewEnumerator10
      _)
    (:NewEnumerator11
      (goto _label_2))
    (:NewEnumerator12
      (goto _label_2))
    (:NewEnumerator13
      _)
    (:NewEnumerator14
      (goto _label_2))
    (:NewEnumerator15
      (goto _label_2)))
  ;[1 1 1] Make South wall
  (switch Utilities|FlowControl|Switch|SwitchonRoomType _roomtype
    (:NewEnumerator0
      _)
    (:NewEnumerator1
      _)
    (:NewEnumerator2
      _)
    (:NewEnumerator3
      (bind _returnvalue_3 (Game|SpawnActorfromClass "/Script/Engine.StaticMeshActor" (Math|Transform|MakeTransform (Math|Vector|MakeVector 0.0 (|((dim/2)+5) _output_get_2) 0.0) "0, 0, 0" (Math|Vector|MakeVector (.x _relativescale3d) 0.1 4.0)) "Undefined" 0 0 :!label _label_3))
      (Transformation|SetMobility _returnvalue_3 "Stationary")
      (Components|StaticMesh|SetStaticMesh (Variables|/Script/Engine.StaticMeshActor|GetStaticMeshComponent _returnvalue_3) "/Game/Shapes/Shape_Cube.Shape_Cube")
      (Rendering|Material|SetMaterial (Variables|/Script/Engine.StaticMeshActor|GetStaticMeshComponent _returnvalue_3) 0 (Variables|Default|GetWallMaterial))
      (Transformation|AttachActorToActor _returnvalue_3 self "None" "KeepRelative" "KeepRelative" "KeepRelative" true)
      (Utilities|Array|Add (Variables|Default|GetWalls) _returnvalue_3))
    (:NewEnumerator4
      _)
    (:NewEnumerator5
      _)
    (:NewEnumerator6
      (goto _label_3))
    (:NewEnumerator7
      _)
    (:NewEnumerator8
      (goto _label_3))
    (:NewEnumerator9
      _)
    (:NewEnumerator10
      (goto _label_3))
    (:NewEnumerator11
      _)
    (:NewEnumerator12
      (goto _label_3))
    (:NewEnumerator13
      (goto _label_3))
    (:NewEnumerator14
      _)
    (:NewEnumerator15
      (goto _label_3)))
  ;[1 1 1] Make West wall
  (switch Utilities|FlowControl|Switch|SwitchonRoomType _roomtype
    (:NewEnumerator2
      _)
    (:NewEnumerator6
      _)
    (:NewEnumerator7
      _)
    (:NewEnumerator9
      _)
    (:NewEnumerator12
      _)
    (:NewEnumerator13
      _)
    (:NewEnumerator14
      _))
  (bind _returnvalue_4 (Game|SpawnActorfromClass "/Script/Engine.StaticMeshActor" (Math|Transform|MakeTransform (Math|Vector|MakeVector (|(5-(dim/2)) _output_get) 0.0 0.0) "0, 0, 0" (Math|Vector|MakeVector 0.1 (.y _relativescale3d) 4.0)) "Undefined" 0 0))
  (Transformation|SetMobility _returnvalue_4 "Stationary")
  (Components|StaticMesh|SetStaticMesh (Variables|/Script/Engine.StaticMeshActor|GetStaticMeshComponent _returnvalue_4) "/Game/Shapes/Shape_Cube.Shape_Cube")
  (Rendering|Material|SetMaterial (Variables|/Script/Engine.StaticMeshActor|GetStaticMeshComponent _returnvalue_4) 0 (Variables|Default|GetWallMaterial))
  (Transformation|AttachActorToActor _returnvalue_4 self "None" "KeepRelative" "KeepRelative" "KeepRelative" true)
  (Utilities|Array|Add (Variables|Default|GetWalls) _returnvalue_4))

(fn DestryoWalls
  ;[1 1 1] Destroys the wall actors - to be called when floor is destroyed
  (for _array_element (Variables|Default|GetWalls)
    (Actor|DestroyActor _array_element)))

(fn SetLava
  (params (CanBeLava :type Boolean) (LavaPercent :type Integer))
  (if CanBeLava
    (if (< (Math|Random|RandomInteger 100) LavaPercent)
      (Rendering|Material|SetMaterial (Variables|Default|GetFloor) 0 "/Game/Materials/LavaMat.LavaMat"))))